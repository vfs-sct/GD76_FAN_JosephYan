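; BP_AISpawner is a placeable actor that spawns a chosen AI class, either on BeginPlay or once when a player overlaps its trigger.
; OnSpawnAI spawns at the actor's location facing AISpawnDirection, then unpossesses and repossesses the pawn to work around a C++ teams bug.
; With an optional patrol path, it sets the AI state and path, and only then fires the spawned event.
; The construction script labels the spawner with its class name.
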(event OnComponentBeginOverlap(SpawnOverlap)
  (params (OverlappedComponent :type Primitive%20Component%20Object%20Reference) (OtherActor :type Actor%20Object%20Reference) (OtherComp :type Primitive%20Component%20Object%20Reference) (OtherBodyIndex :type Integer) (bFromSweep :type Boolean) (SweepResult :type Hit%20Result%20Structure%20%28by%20ref%29))
  ;[1 1 1] If spawn method is set to overlap
  (switch Utilities|FlowControl|Switch|SwitchonEN_AISpawnMethod (Variables|Default|Get_aiSpawnMethod)
    (:NewEnumerator2
      (Utilities|IsPlayer OtherActor
        (:true
          (Utilities|FlowControl|DoOnce false
            (:Completed
              (CallFunction|OnSpawnAI))))))))

(event EventBeginPlay
  ;[1 1 1] If spawn method is set to begin play
  (switch Utilities|FlowControl|Switch|SwitchonEN_AISpawnMethod (Variables|Default|Get_aiSpawnMethod)
    (:NewEnumerator0
      (CallFunction|OnSpawnAI))))

(fn ConstructionScript
  (CallFunction|SetPreviewName))

(fn OnSpawnAI
  (bind __optionalstartingpatrolpath (Variables|Default|Get_optionalStartingPatrolPath))
  (bind _returnvalue (AI|SpawnAIFromClass (Variables|Default|Get_aiToSpawn) 0 (Transformation|GetActorLocation) (Transformation|GetWorldRotation (Variables|Default|GetAISpawnDirection)) true 0)) ; No need to feed in a tree here, the AI class\nsets the tree appropriate for it on initialize
  (bind _asbp_base_aicharacter (Utilities|Casting|CastToBP_BaseAICharacter _returnvalue)
    (:then
      (bind _asbp_base_aicontroller (Utilities|Casting|CastToBP_BaseAIController (Pawn|GetController _asbp_base_aicharacter)))
      (Pawn|UnPossess _asbp_base_aicontroller) ; The C++ code for teams\nleft an issue on SpawnAI\nmethod call. Clear, then\nreposses. Hack fix.
      (Pawn|Possess _asbp_base_aicontroller _asbp_base_aicharacter)
      ;[1 1 1] Start on patrol if Spawner has a patrol point
      (Utilities|IsValid __optionalstartingpatrolpath
        (:Is%20Valid
          (Default|SetAIState _asbp_base_aicontroller "NewEnumerator2")
          (Default|SetPatrolPath _asbp_base_aicharacter __optionalstartingpatrolpath)
          (Default|CallOnAISpawnedEvent _asbp_base_aicharacter _asbp_base_aicontroller))
        (:Is%20Not%20Valid
          _)))
    (:CastFailed
      (Development|PrintString "ERROR: SPAWN NULL FROM BP_AISPAWNER INSTANCE" true true "(R=1.000000,G=0.000000,B=0.018907,A=1.000000)" 1e+01)))
  (return _asbp_base_aicharacter _asbp_base_aicontroller))

(fn SetStartingPatrolPoint
  (params (_optionalStartingPatrolPath :type BP%20Patrol%20Path%20Object%20Reference))
  (Variables|Default|Set_optionalStartingPatrolPath _optionalStartingPatrolPath))

(fn SetAIClasstoSpawn
  (params (_aiToSpawn :type BP%20Base%20AI%20Character%20Class%20Reference))
  (Variables|Default|Set_aiToSpawn _aiToSpawn))

(fn SetPreviewName
  (bind __aitospawn (Variables|Default|Get_aiToSpawn))
  (if (Utilities|IsValidClass __aitospawn)
    (LocalVariables|Set_text (Utilities|Text|ToText(String) (Utilities|String|Append "Spawner:" "  
" (Utilities|GetClassDisplayName __aitospawn))))
    (Rendering|Components|TextRender|SetText (Variables|Default|GetNameOfClass) (LocalVariables|Get_text))
    (else
      (LocalVariables|Set_text ""))))