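; BP_DetectDirection is a utility trigger that reports which side the player leaves it from.
; When an actor ends overlap with its Box and passes the player check, its distances to the Forward and Backward marker components are compared.
; The nearer marker decides whether it calls OnPlayerLeavingForward or OnPlayerLeavingBackward, passing the player along.
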(event OnComponentEndOverlap(Box)
  (params (OverlappedComponent :type Primitive%20Component%20Object%20Reference) (OtherActor :type Actor%20Object%20Reference) (OtherComp :type Primitive%20Component%20Object%20Reference) (OtherBodyIndex :type Integer))
  (CallFunction|CheckPlayerLeavingDirection OtherActor))

(fn ConstructionScript)

(fn CheckPlayerLeavingDirection
  (params (Actor :type Actor%20Object%20Reference))
  (bind _returnvalue (Transformation|GetActorLocation Actor))
  (bind _playercharacter (Utilities|IsPlayer Actor)
    (:true
      (if (< (Math|Vector|Distance(Vector) (Transformation|GetWorldLocation (Variables|Default|GetForward)) _returnvalue) (Math|Vector|Distance(Vector) _returnvalue (Transformation|GetWorldLocation (Variables|Default|GetBackward))))
        (Default|CallOnPlayerLeavingForward _playercharacter)
        (else
          (Default|CallOnPlayerLeavingBackward _playercharacter))))))