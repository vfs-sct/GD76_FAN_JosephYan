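; Interactable sphere Blueprint that smoothly cycles its material through preset primary and secondary color pairs each time it is interacted with.
; The construction script creates a dynamic material instance, so each sphere changes color independently.
; On interact, it captures the current colors, picks the next pair from parallel arrays and advances the index, wrapping on the primary array's length.
; A timeline then lerps both vector parameters to the new colors.
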(event Custom|UpdateColors
  (bind _returnvalue (Rendering|Material|GetVectorParameterValue (Variables|Default|Get_dynamicMaterialInstance) (Variables|Default|Get_primaryColorParamKey) :!class /Script/Engine.MaterialInstanceDynamic))
  (Variables|Default|Set_currentPrimaryColor _returnvalue)
  (bind _returnvalue_2 (Rendering|Material|GetVectorParameterValue (Variables|Default|Get_dynamicMaterialInstance) (Variables|Default|Get_secondaryColorParamKey) :!class /Script/Engine.MaterialInstanceDynamic))
  (Variables|Default|Set_currentSecondaryColor _returnvalue_2)
  (Variables|Default|Set_nextPrimaryColor (Utilities|Array|Get(acopy) (Variables|Default|Get_primaryColors) (Variables|Default|Get_materialColorIndex)))
  (Variables|Default|Set_nextSecondaryColor (Utilities|Array|Get(acopy) (Variables|Default|Get_secondaryColors) (Variables|Default|Get_materialColorIndex)))
  (CallFunction|IncrementColorIndex)
  (bind _alpha (Timeline|UpdateColor%20Timeline PlayFromStart)
    (:Update
      (Rendering|Material|SetVectorParameterValue (Variables|Default|Get_dynamicMaterialInstance) (Variables|Default|Get_primaryColorParamKey) (Math|Color|Lerp(LinearColor) (Variables|Default|Get_currentPrimaryColor) (Variables|Default|Get_nextPrimaryColor) _alpha) :!class /Script/Engine.MaterialInstanceDynamic)
      (Rendering|Material|SetVectorParameterValue (Variables|Default|Get_dynamicMaterialInstance) (Variables|Default|Get_secondaryColorParamKey) (Math|Color|Lerp(LinearColor) (Variables|Default|Get_currentSecondaryColor) (Variables|Default|Get_nextSecondaryColor) _alpha) :!class /Script/Engine.MaterialInstanceDynamic))))

(event EventOnInteract
  (params (playerCharacter :type BP%20Base%20Player%20Character%20Object%20Reference))
  (CallFunction|UpdateColors))

(fn ConstructionScript
  ;[0.15 0.15 0.15 0.5] Create a dynamic material so we can call code on it to change it on runtime, without changes the other copies of the same material objects.
  (bind _returnvalue (Rendering|Material|CreateDynamicMaterialInstance (Variables|Default|GetSphere) 0 0 "None" :!class /Script/Engine.PrimitiveComponent))
  (Variables|Default|Set_dynamicMaterialInstance _returnvalue))

(fn IncrementColorIndex
  ;[0.15 0.15 0.15 0.5] Increment current material index value. Reset to 0 if over or equal to length of materials.
  (bind _result (Math|Integer|IncrementInt (Variables|Default|Get_materialColorIndex))
    (:%20%20
      (if (>= _result (Utilities|Array|Length (Variables|Default|Get_primaryColors)))
        (Variables|Default|Set_materialColorIndex 0)))))